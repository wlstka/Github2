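; Lobby game mode that registers joining players, marks the first as host and spawns their lobby character at a PlayerStart.
; Keeps a GUID-keyed user info array; setters for number, ready state and character choice copy it to BP_LobbyGS.
; A ForLoopAllPC macro tells each lobby controller to refresh or move into the game.
; Logout resets everyone's ready state after a delay, without removing the array entry.
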(event `self.K2_PostLogin`
  (params (NewPlayer :type "PlayerController Object Reference"))
  (bind _asbp_lobby_pc (cast `/Game/Blueprints/PlayerController/BP_LobbyPC` NewPlayer))
  (set `self.CurrentLobbyPC` _asbp_lobby_pc)
  (`|ExecutionSequence`
    (:`then_0`
      (`self.Set User Info`))
    (:`then_1`
      (`self.SpawnCharacterAnimation` "/Game/Character/PlayerCharacter/LobbyPlayerCharacter/BP_LobbyCharacter.BP_LobbyCharacter_C" (`self.CurrentLobbyPC`)))))

(event `self.K2_OnLogout`
  (params (ExitingController :type "Controller Object Reference"))
  (`KismetSystemLibrary.Delay` 1.0)
  (`self.ResetUserList`))

(fn `BoolGuid`
  (params (InGuid :type "Guid Structure (by ref)"))
  (returns (OutCurrentPlayerInfo :type "/Game/Structs/S_UserInfo Structure") (OutCurrentPlayerIndex :type Integer) (ReturnValue :type Boolean))
  (locals (CurrentPlayerInfo :type "/Game/Structs/S_UserInfo Structure") (CurrentPlayerIndex :type Integer))
  (for (_array_element _array_index) (`self.GM_UserInfoArr`)
    (bind _output_get (set `local.CurrentPlayerInfo` _array_element))
    (set `local.CurrentPlayerIndex` _array_index)
    (bind _returnvalue (== (`.PlayerGuid_9_C3A7860141F0A9A5432560B79025DBC0` (break `/Game/Structs/S_UserInfo` _output_get)) (`local.InGuid`)))
    (if _returnvalue
      (return (`local.CurrentPlayerInfo`) (`local.CurrentPlayerIndex`) _returnvalue))))

(fn `GameStart`
  (locals (NewLocalVar_0 :type String :default "ServerTravel /Game/Maps/InGame"))
  (bind _asbp_lobby_pc (`self.ForLoopAllPC`)
    (:`LoopBody`
      (`/Game/Blueprints/PlayerController/BP_LobbyPC.Owner_MoveToInGame` _asbp_lobby_pc))))

(fn `GetLobbyGS`
  (returns (`AsBP Lobby GS` :type "/Game/Blueprints/GameState/BP_LobbyGS Object Reference"))
  (bind _asbp_lobby_gs (cast `/Game/Blueprints/GameState/BP_LobbyGS` (`GameplayStatics.GetGameState`)))
  (return _asbp_lobby_gs))

(fn `GetLobbyPC`
  (params (PlayerIndex :type Integer))
  (returns (`AsBP Lobby PC` :type "/Game/Blueprints/PlayerController/BP_LobbyPC Object Reference"))
  (bind _asbp_lobby_pc (cast `/Game/Blueprints/PlayerController/BP_LobbyPC` (`GameplayStatics.GetPlayerController` PlayerIndex)))
  (return _asbp_lobby_pc))

(fn `ResetUserList`
  (`|ExecutionSequence`
    (:`then_0`
      (bind _asbp_lobby_pc (`self.ForLoopAllPC`)
        (:`LoopBody`
          (set `/Game/Blueprints/PlayerState/BP_LobbyPS.IsReady` false (`/Game/Blueprints/PlayerController/BP_LobbyPC.GetLobbyPS` _asbp_lobby_pc))
          (`/Game/Blueprints/PlayerController/BP_LobbyPC.Owner_UpdateUserReady` _asbp_lobby_pc))))
    (:`then_2`
      (for _array_element (`self.GM_UserInfoArr`)
        (setmembers `/Game/Structs/S_UserInfo` :`StructRef` _array_element :`PlayerIsReady` false)))
    (:`then_3`
      (`self.UpdateUserList`))))

(fn `Set User Info`
  (`|ExecutionSequence`
    (:`then_0`
      (`self.Set User Info Guid`))
    (:`then_1`
      (`/Game/Blueprints/PlayerController/BP_LobbyPC.OwnerSetNickName` (`self.CurrentLobbyPC`)))
    (:`then_2`
      (`/Game/Blueprints/PlayerController/BP_LobbyPC.ServerSetUserNum` (`self.CurrentLobbyPC`) (+ (`self.CurrentLobbyPCNum`) 1)))
    (:`then_3`
      (bind _returnvalue (`self.GetNumPlayers`))
      (if (== _returnvalue 1)
        (set `/Game/Blueprints/PlayerController/BP_LobbyPC.Is Host` true (`self.CurrentLobbyPC`))))))

(fn `Set User Info Guid`
  (locals (NewGuid :type "Guid Structure") (NewUserInfo :type "/Game/Structs/S_UserInfo Structure"))
  (set `local.NewGuid` (`KismetGuidLibrary.NewGuid`))
  (set `local.NewUserInfo` (make `/Game/Structs/S_UserInfo` :`PlayerGuid` (`local.NewGuid`) :`PlayerLobbyPC` (`self.CurrentLobbyPC`)))
  (bind _returnvalue (`KismetArrayLibrary.Array_Add` (`self.GM_UserInfoArr`) (`local.NewUserInfo`)))
  (set `self.CurrentLobbyPCNum` _returnvalue)
  (`/Game/Blueprints/PlayerController/BP_LobbyPC.SetGuid` (`self.CurrentLobbyPC`) (`.PlayerGuid_9_C3A7860141F0A9A5432560B79025DBC0` (break `/Game/Structs/S_UserInfo` (`local.NewUserInfo`)))))

(fn `Set User Info NickName`
  (params (InGuid :type "Guid Structure") (InNickName :type String))
  (locals (CurrentPlayerInfo :type "/Game/Structs/S_UserInfo Structure"))
  (bind (_outcurrentplayerinfo _outcurrentplayerindex _returnvalue) (`self.BoolGuid` InGuid))
  (if _returnvalue
    (setmembers `/Game/Structs/S_UserInfo` :`StructRef` (`|GetArrayItem` (`self.GM_UserInfoArr`) _outcurrentplayerindex) :`PlayerNickName` (`local.InNickName`))))

(fn `Set User Select Character`
  (params (InGuid :type "Guid Structure (by ref)") (InClass :type "/Game/Enum/EPlayerClass Enum" :default "NewEnumerator2"))
  (bind (_outcurrentplayerinfo _outcurrentplayerindex _returnvalue) (`self.BoolGuid` InGuid))
  (if _returnvalue
    (setmembers `/Game/Structs/S_UserInfo` :`StructRef` (`|GetArrayItem` (`self.GM_UserInfoArr`) _outcurrentplayerindex) :`EClass` (`local.InClass`))
    (`/Game/Blueprints/GameState/BP_LobbyGS.Update Player Info` (`self.GetLobbyGS`) (`self.GM_UserInfoArr`))
    (`self.UpdateUserSelctCharacter`)))

(fn `SetUserInfoNum`
  (params (InGuid :type "Guid Structure") (InNum :type Integer))
  (locals (CurrentPlayerInfo :type "/Game/Structs/S_UserInfo Structure"))
  (bind (_outcurrentplayerinfo _outcurrentplayerindex _returnvalue) (`self.BoolGuid` InGuid))
  (if _returnvalue
    (setmembers `/Game/Structs/S_UserInfo` :`StructRef` (`|GetArrayItem` (`self.GM_UserInfoArr`) _outcurrentplayerindex) :`PlayerNum` (`local.InNum`))
    (`/Game/Blueprints/GameState/BP_LobbyGS.Update Player Info` (`self.GetLobbyGS`) (`self.GM_UserInfoArr`))
    (`self.UpdateUserList`)
    (return)))

(fn `SetUserReady`
  (params (InReady :type Boolean) (InGuid :type "Guid Structure"))
  (locals (CurrentPlayerInfo :type "/Game/Structs/S_UserInfo Structure"))
  (bind (_outcurrentplayerinfo _outcurrentplayerindex _returnvalue) (`self.BoolGuid` InGuid))
  (if _returnvalue
    (setmembers `/Game/Structs/S_UserInfo` :`StructRef` (`|GetArrayItem` (`self.GM_UserInfoArr`) _outcurrentplayerindex) :`PlayerIsReady` (`local.InReady`))
    (`/Game/Blueprints/GameState/BP_LobbyGS.Update Player Info` (`self.GetLobbyGS`) (`self.GM_UserInfoArr`))
    (`self.UpdateUserReadyState`)))

(fn `SpawnCharacterAnimation`
  (params (InClass :type "/Game/Character/PlayerCharacter/LobbyPlayerCharacter/BP_LobbyCharacter Class Reference") (InPC :type "/Game/Blueprints/PlayerController/BP_LobbyPC Object Reference"))
  (bind _returnvalue (`GameplayStatics.GetActorOfClass` "/Script/Engine.PlayerStart"))
  (bind _returnvalue_2 (`|SpawnActorFromClass` (`local.InClass`) (`self.GetTransform` _returnvalue) "AlwaysSpawn" "OverrideRootScale" (`local.InPC`) null))
  (`Controller.Possess` (`local.InPC`) _returnvalue_2))

(fn `UpdateCharacterAnimaion`
  (params (InPC :type "/Game/Blueprints/PlayerController/BP_LobbyPC Object Reference") (InClass :type "/Game/Character/PlayerCharacter/LobbyPlayerCharacter/BP_LobbyCharacter Class Reference"))
  (`self.K2_DestroyActor` (`Controller.K2_GetPawn` InPC))
  (`self.SpawnCharacterAnimation` (`local.InClass`) (`local.InPC`)))

(fn `UpdateUserList`
  (bind _asbp_lobby_pc (`self.ForLoopAllPC`)
    (:`LoopBody`
      (`/Game/Blueprints/PlayerController/BP_LobbyPC.OwnerUpdateUserList` _asbp_lobby_pc))))

(fn `UpdateUserReadyState`
  (bind _asbp_lobby_pc (`self.ForLoopAllPC`)
    (:`LoopBody`
      (`/Game/Blueprints/PlayerController/BP_LobbyPC.Owner_UpdateUserReady` _asbp_lobby_pc))))

(fn `UpdateUserSelctCharacter`
  (bind _asbp_lobby_pc (`self.ForLoopAllPC`)
    (:`LoopBody`
      (`/Game/Blueprints/PlayerController/BP_LobbyPC.Owner_UpdateUserSelectCharacter` _asbp_lobby_pc))))

(fn `UserConstructionScript`
  (`parent.UserConstructionScript`))