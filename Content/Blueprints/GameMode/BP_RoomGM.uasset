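; Game mode for a multiplayer room that sets up joining players and tracks whether the game has started.
; On login it has the new BP_RoomPC load its nickname from save and makes it host if it is the only player.
; Helpers use a macro over all room controllers to refresh names and player lists.
; An older GUID and timer-based registration flow remains in the graph, disconnected.
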(event `self.ReceiveTick`
  (params (DeltaSeconds :type "Float (single-precision)")))

(event `GameStart`
  (set `self.IsStarted` true))

(event `self.K2_PostLogin`
  (params (NewPlayer :type "PlayerController Object Reference"))
  (bind _asbp_room_pc (cast `/Game/Blueprints/PlayerController/BP_RoomPC` NewPlayer))
  (set `self.CurrentRoomPC` _asbp_room_pc)
  (`|ExecutionSequence`
    (:`then_0`
      (`/Game/Blueprints/PlayerController/BP_RoomPC.OwnerUpdatePlayerNickNameFromSave` (`self.CurrentRoomPC`)))
    (:`then_1`
      (`self.SetInitPlayerHost`))))

(fn `GetRoomGS`
  (returns (`AsBP Room GS` :type "/Game/Blueprints/GameState/BP_RoomGS Object Reference"))
  (bind _asbp_room_gs (cast `/Game/Blueprints/GameState/BP_RoomGS` (`GameplayStatics.GetGameState`)))
  (return _asbp_room_gs))

(fn `Set Player Nick Name`
  (params (InGuid :type "Guid Structure") (InNickName :type String))
  (locals (CurrentPlayerInfo :type "/Game/Structs/S_UserInfo Structure") (CurrentPlayerIndex :type Integer))
  (for (_array_element _array_index) (`self.FCurrentNewPlayerInfoArr`)
    (bind _output_get (set `local.CurrentPlayerInfo` _array_element))
    (set `local.CurrentPlayerIndex` _array_index)
    (if (== (`.PlayerGuid_9_C3A7860141F0A9A5432560B79025DBC0` (break `/Game/Structs/S_UserInfo` _output_get)) (`local.InGuid`))
      (setmembers `/Game/Structs/S_UserInfo` :`StructRef` (`|GetArrayItem` (`self.FCurrentNewPlayerInfoArr`) (`local.CurrentPlayerIndex`)) :`PlayerNickName` (`local.InNickName`))
      (`self.UpdatePlayerInfo`)
      (return))))

(fn `SetInitPlayerHost`
  (bind _returnvalue (`self.GetNumPlayers`))
  (if (== _returnvalue 1)
    (set `/Game/Blueprints/PlayerController/BP_RoomPC.IsHost` true (`self.CurrentRoomPC`))))

(fn `SetPlayerGuid`
  (if (and (`KismetSystemLibrary.IsValid` (`self.CurrentRoomPC`)) (`KismetSystemLibrary.IsValid` (`self.GetRoomGS`)))
    (set `self.NewGuid` (`KismetGuidLibrary.NewGuid`))
    (set `self.FCurrentNewPlayerInfo` (make `/Game/Structs/S_UserInfo` :`PlayerGuid` (`self.NewGuid`) :`PlayerRoomPC` (`self.CurrentRoomPC`)))
    (`KismetArrayLibrary.Array_Add` (`self.FCurrentNewPlayerInfoArr`) (`self.FCurrentNewPlayerInfo`))
    (`/Game/Blueprints/PlayerController/BP_RoomPC.SetGuid` (`self.CurrentRoomPC`) (`.PlayerGuid_9_C3A7860141F0A9A5432560B79025DBC0` (break `/Game/Structs/S_UserInfo` (`self.FCurrentNewPlayerInfo`))))
    (`/Game/Blueprints/GameState/BP_RoomGS.UpdatePlayerInfo` (`self.GetRoomGS`) (`self.FCurrentNewPlayerInfoArr`))))

(fn `SetPlayerInfo`
  (`KismetSystemLibrary.K2_ClearAndInvalidateTimerHandle` (`self.TH_SetPlayerInfo`))
  (bind _asbp_room_pc (`self.ForEachAllRoomPC`)
    (:`LoopBody`
      (`/Game/Blueprints/PlayerController/BP_RoomPC.OwnerdSetPlayerInfo` _asbp_room_pc))))

(fn `UpdatePlayerInfo`
  (bind _asbp_room_pc (`self.ForEachAllRoomPC`)
    (:`LoopBody`
      (`/Game/Blueprints/PlayerController/BP_RoomPC.OwnerUpdatePlayerList` _asbp_room_pc))))

(fn `UpdatePlayerNickName`
  (bind _asbp_room_pc (`self.ForEachAllRoomPC`)
    (:`LoopBody`
      (`/Game/Blueprints/PlayerController/BP_RoomPC.OwnerUpdatePlayerNickNameFromSave` _asbp_room_pc))
    (:`Completed`
      (`KismetSystemLibrary.K2_ClearAndInvalidateTimerHandle` (`self.TH_UpdateNickName`)))))

(fn `UserConstructionScript`
  (`parent.UserConstructionScript`))