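; In-game GameMode Blueprint that sets up each player on login and loads saved user info into the game state.
; PostLogin spawns a BP_InGamePawn at a found PlayerStart for controllers lacking a pawn, possesses it and calls ServerInitPlayer.
; It then copies UserInfo from BattleEndedGameInstance's save data into BP_InGameGS.
; Helpers provide typed controller and game state getters, plus a loop over all player controllers.
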(event `self.K2_PostLogin`
  (params (NewPlayer :type "PlayerController Object Reference"))
  ;[1 1 1] 로그인
  (`|ExecutionSequence`
    (:`then_0`
      (bind _asbp_in_game_pc (cast `/Game/Blueprints/PlayerController/BP_InGamePC` NewPlayer))
      (set `self.CurrentInGamePC` _asbp_in_game_pc)
      (`/Engine/EditorBlueprintResources/StandardMacros.IsValid` (`Controller.K2_GetPawn` (`self.CurrentInGamePC`))
        (:`Is Not Valid`
          (bind _returnvalue (`GameplayStatics.GetActorOfClass` "/Script/Engine.PlayerStart"))
          (bind _returnvalue_2 (`|SpawnActorFromClass` "/Game/Character/BP_InGamePawn.BP_InGamePawn_C" (`self.GetTransform` _returnvalue) "Undefined" "OverrideRootScale" (`self.CurrentInGamePC`) null))
          (`Controller.Possess` (`self.CurrentInGamePC`) _returnvalue_2)
          (`/Game/Blueprints/PlayerController/BP_InGamePC.Server_InitPlayer` (`self.CurrentInGamePC`)))))
    (:`then_1`
      (bind _asbattle_ended_game_instance (cast `/Game/Blueprints/BattleEndedGameInstance` (`GameplayStatics.GetGameInstance`)))
      (bind _userinfogs (`/Game/Blueprints/BattleEndedGameInstance.GetUserInfoFromSaveGS` _asbattle_ended_game_instance))
      (set `/Game/Blueprints/GameState/BP_InGameGS.UserInfo` _userinfogs (`self.GetInGameGS`)))))

(fn `GetInGameGS`
  (returns (`AsBP in Game GS` :type "/Game/Blueprints/GameState/BP_InGameGS Object Reference"))
  (bind _asbp_in_game_gs (cast `/Game/Blueprints/GameState/BP_InGameGS` (`GameplayStatics.GetGameState`)))
  (return _asbp_in_game_gs))

(fn `GetInGamePC`
  (params (PlayerIndex :type Integer))
  (returns (`AsBP in Game PC` :type "/Game/Blueprints/PlayerController/BP_InGamePC Object Reference"))
  (bind _asbp_in_game_pc (cast `/Game/Blueprints/PlayerController/BP_InGamePC` (`GameplayStatics.GetPlayerController` PlayerIndex)))
  (return _asbp_in_game_pc))

(fn `UserConstructionScript`
  (`parent.UserConstructionScript`))