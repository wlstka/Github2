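; Game instance Blueprint that persists player info through save games and handles level travel to an IP address or the Title level.
; Nickname, per-user info and a separate BP_SaveGS UserInfo record each use their own slot.
; Joining saves the nickname, then opens the IP as a level unless IsStarted is set.
; SaveUserInfo saves by user number, but its getter always loads index 0 and only prints, leaving its return unreached.
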(fn `GetNickNameFromSaveInfo`
  (returns (NickName :type String))
  (bind _returnvalue (`GameplayStatics.LoadGameFromSlot` "NickName"))
  (bind _asbp_user_info_save_game (cast `/Game/Save/BP_UserInfoSaveGame` _returnvalue))
  (return (`/Game/Save/BP_UserInfoSaveGame.NickName` _asbp_user_info_save_game)))

(fn `GetUserInfoFromSaveGS`
  (returns (UserInfoGS :type "Array of /Game/Structs/FUserInfo Structure"))
  (bind _returnvalue (`GameplayStatics.LoadGameFromSlot` "UserInfoGS"))
  (`KismetSystemLibrary.PrintString` (`KismetSystemLibrary.GetDisplayName` _returnvalue) true true (struct :`G` 0.66 :`B` 1.0 :`A` 1.0) 666.0)
  (bind _asbp_save_gs (cast `/Game/Save/BP_SaveGS` _returnvalue))
  (return (`/Game/Save/BP_SaveGS.UserInfo` _asbp_save_gs)))

(fn `GetUserInfoFromSaveInfo`
  (params (InNum :type Integer))
  (returns (NickName :type String) (Guid :type "Guid Structure") (Class :type "/Game/Enum/EPlayerClass Enum") (Num :type Integer))
  (bind _returnvalue (`GameplayStatics.LoadGameFromSlot` "UserInfo"))
  (bind _asbp_user_info_save_game (cast `/Game/Save/BP_UserInfoSaveGame` _returnvalue))
  (`KismetSystemLibrary.PrintString` (`KismetStringLibrary.Concat_StrStr` (`/Game/Save/BP_UserInfoSaveGame.NickName` _asbp_user_info_save_game) (`KismetStringLibrary.Conv_IntToString` (`/Game/Save/BP_UserInfoSaveGame.Num` _asbp_user_info_save_game)) (`KismetGuidLibrary.Conv_GuidToString` (`/Game/Save/BP_UserInfoSaveGame.Guid` _asbp_user_info_save_game)) (`|GetEnumeratorNameAsString` (`/Game/Save/BP_UserInfoSaveGame.Class` _asbp_user_info_save_game))) true true (struct :`G` 0.66 :`B` 1.0 :`A` 1.0) 50.0))

(fn `MoveToNewLevel`
  (params (InIP :type String) (InNickName :type String))
  (returns (IsStarted :type Boolean))
  (if (not (`self.IsStarted`))
    (`self.SaveUserNickName` InNickName)
    (`GameplayStatics.OpenLevel` (`KismetStringLibrary.Conv_StringToName` (`local.InIP`)))
    (else
      (return (`self.IsStarted`)))))

(fn `MoveToTitle`
  (`GameplayStatics.OpenLevel` "Title"))

(fn `SaveUserInfo`
  (params (InNickName :type String) (InGuid :type "Guid Structure") (InClass :type "/Game/Enum/EPlayerClass Enum" :default "NewEnumerator2") (InNum :type Integer))
  (bind _output_get (set `self.Number` InNum))
  (`KismetSystemLibrary.PrintString` (`KismetStringLibrary.Conv_IntToString` _output_get) true true (struct :`G` 0.66 :`B` 1.0 :`A` 1.0) 100.0)
  (if (not (`KismetSystemLibrary.IsValid` (`self.UserInfoSaveGame`)))
    (bind _returnvalue (`GameplayStatics.CreateSaveGameObject` "/Game/Save/BP_UserInfoSaveGame.BP_UserInfoSaveGame_C"))
    (set `self.UserInfoSaveGame` _returnvalue))
  (`|ExecutionSequence`
    (:`then_0`
      (set `/Game/Save/BP_UserInfoSaveGame.NickName` (`local.InNickName`) (`self.UserInfoSaveGame`)))
    (:`then_1`
      (set `/Game/Save/BP_UserInfoSaveGame.Guid` (`local.InGuid`) (`self.UserInfoSaveGame`)))
    (:`then_2`
      (set `/Game/Save/BP_UserInfoSaveGame.Class` (`local.InClass`) (`self.UserInfoSaveGame`)))
    (:`then_3`
      (set `/Game/Save/BP_UserInfoSaveGame.Num` (`local.InNum`) (`self.UserInfoSaveGame`)))
    (:`then_4`
      (`GameplayStatics.SaveGameToSlot` (`self.UserInfoSaveGame`) "UserInfo" (`self.Number`)))))

(fn `SaveUserNickName`
  (params (InNickName :type String))
  (if (not (`KismetSystemLibrary.IsValid` (`self.UserInfoSaveGame`)))
    (bind _returnvalue (`GameplayStatics.CreateSaveGameObject` "/Game/Save/BP_UserInfoSaveGame.BP_UserInfoSaveGame_C"))
    (set `self.UserInfoSaveGame` _returnvalue))
  (`|ExecutionSequence`
    (:`then_0`
      (set `/Game/Save/BP_UserInfoSaveGame.NickName` (`local.InNickName`) (`self.UserInfoSaveGame`))
      (`GameplayStatics.SaveGameToSlot` (`self.UserInfoSaveGame`) "NickName"))))

(fn `ServerSaveGS`
  (params (InUserInfo :type "Array of /Game/Structs/FUserInfo Structure"))
  (if (not (`KismetSystemLibrary.IsValid` (`self.SaveGS`)))
    (bind _returnvalue (`GameplayStatics.CreateSaveGameObject` "/Game/Save/BP_SaveGS.BP_SaveGS_C"))
    (set `self.SaveGS` _returnvalue))
  (set `/Game/Save/BP_SaveGS.UserInfo` (`local.InUserInfo`) (`self.SaveGS`))
  (`GameplayStatics.SaveGameToSlot` (`self.SaveGS`) "UserInfoGS"))