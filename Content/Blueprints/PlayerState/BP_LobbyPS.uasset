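; Lobby player state holding a player's nickname, ready flag, order number and selected character class.
; Server events set the ready flag and class.
; RepNotifies forward each change to server functions on BP_LobbyPC, fetched via player controller index 0.
; Nickname, ready and order updates pass that controller's PlayerGuid, while class selection passes this state's own Guid.
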(event `Server_UpdateIsReady`
  (params (IsReady :type Boolean))
  (`self.UpdateIsReady` IsReady))

(event `Server_UpdateSelectCharacter`
  (params (EPlayerClass :type "/Game/Enum/EPlayerClass Enum" :default "NewEnumerator2"))
  (`self.UpdateSelectCharacter` EPlayerClass))

(fn `GetLobbyPC`
  (returns (`AsBP Lobby PC` :type "/Game/Blueprints/PlayerController/BP_LobbyPC Object Reference"))
  (bind _asbp_lobby_pc (cast `/Game/Blueprints/PlayerController/BP_LobbyPC` (`GameplayStatics.GetPlayerController` 0)))
  (return _asbp_lobby_pc))

(fn `OnRep_EPlayerClass`
  (`/Game/Blueprints/PlayerController/BP_LobbyPC.Server_PlayerCharacterSelect` (`self.GetLobbyPC`) (`self.Guid`) (`self.EPlayerClass`)))

(fn `OnRep_IsReady`
  (bind _asbp_lobby_pc (`self.GetLobbyPC`))
  (`/Game/Blueprints/PlayerController/BP_LobbyPC.Server_UpdateReady` _asbp_lobby_pc (`self.IsReady`) (`/Game/Blueprints/PlayerController/BP_LobbyPC.Player Guid` _asbp_lobby_pc)))

(fn `OnRep_NickName`
  (bind _asbp_lobby_pc (`self.GetLobbyPC`))
  (`/Game/Blueprints/PlayerController/BP_LobbyPC.ServerUpdateUserList` _asbp_lobby_pc (`/Game/Blueprints/PlayerController/BP_LobbyPC.Player Guid` _asbp_lobby_pc) (`self.NickName`)))

(fn `OnRep_NumOrder`
  (bind _asbp_lobby_pc (`self.GetLobbyPC`))
  (`/Game/Blueprints/PlayerController/BP_LobbyPC.ServerUpdateUserNum` _asbp_lobby_pc (`/Game/Blueprints/PlayerController/BP_LobbyPC.Player Guid` _asbp_lobby_pc) (`self.NumOrder`)))

(fn `UpdateIsReady`
  (params (IsReady :type Boolean))
  (set `self.IsReady` IsReady))

(fn `UpdateSelectCharacter`
  (params (EPlayerClass :type "/Game/Enum/EPlayerClass Enum" :default "NewEnumerator2"))
  (set `self.EPlayerClass` EPlayerClass))

(fn `UserConstructionScript`
  (`parent.UserConstructionScript`))