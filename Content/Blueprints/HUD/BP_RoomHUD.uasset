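; Room HUD Blueprint that shows the WBP_RoomHUD widget and relays player-info updates to it.
; BeginPlay creates the widget, adds it to the viewport, and switches to UI-only input with a visible cursor.
; UpdatePlayerInfo forwards to the widget, retrying after a short delay until the widget is valid.
; EnterRoom is empty, and a similar retry chain calling CreatePlayerInfo is disconnected, so it never runs.
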(event `self.ReceiveBeginPlay`
  (bind _returnvalue (`|CreateWidget` "/Game/UI/RoomUI/WBP_RoomHUD.WBP_RoomHUD_C" (`GameplayStatics.GetPlayerController` 0)))
  (bind _output_get (set `self.WBP_RoomHUD` _returnvalue))
  (`UserWidget.AddToViewport` _output_get 0)
  (`WidgetBlueprintLibrary.SetInputMode_UIOnlyEx` (`GameplayStatics.GetPlayerController` 0) _output_get)
  (set `PlayerController.bShowMouseCursor` true (`GameplayStatics.GetPlayerController` 0)))

(event `EnterRoom`)

(event `UpdatePlayerInfo`
  (bind _wbp_roomhud (`self.WBP_RoomHUD`)
    (:`then`
      (`/Game/UI/RoomUI/WBP_RoomHUD.UpdatePlayerInfo` _wbp_roomhud))
    (:`else`
      (`KismetSystemLibrary.Delay` 0.2)
      (`self.UpdatePlayerInfo`))))

(fn `UserConstructionScript`
  (`parent.UserConstructionScript`))