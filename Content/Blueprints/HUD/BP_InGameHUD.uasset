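; In-game HUD Blueprint that puts the WBP_InGameHUD widget on the player's screen.
; On BeginPlay it creates the widget for the owning player controller, stores the reference and adds it to the viewport.
; Nodes for game-only input mode and hiding the mouse cursor are present but unconnected, so they never run.
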(event `self.ReceiveBeginPlay`
  (`|ExecutionSequence`
    (:`then_0`
      (bind _returnvalue (`|CreateWidget` "/Game/UI/InGameUI/WBP_InGameHUD.WBP_InGameHUD_C" (`self.GetOwningPlayerController`)))
      (bind _output_get (set `self.WBP_InGameHUD` _returnvalue))
      (`UserWidget.AddToViewport` _output_get 0))))

(fn `UserConstructionScript`
  (`parent.UserConstructionScript`))