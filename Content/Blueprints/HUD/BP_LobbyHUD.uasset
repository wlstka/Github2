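; Lobby HUD that creates the WBP_LobbyHUD widget on BeginPlay and switches the player to UI-only input with a visible cursor.
; It forwards user info, ready state, host and character selection updates to that widget.
; Each update sets a short timer to retry by function name if the widget is not yet valid.
; SetHostUI's retry names "SetHost" instead of itself, unlike the others.
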(event `self.ReceiveBeginPlay`
  (`parent.ReceiveBeginPlay`)
  (bind _returnvalue (`|CreateWidget` "/Game/UI/LobbyUI/WBP_LobbyHUD.WBP_LobbyHUD_C" (`GameplayStatics.GetPlayerController` 0)))
  (bind _output_get (set `self.WBP_LobbyHUD` _returnvalue))
  (`UserWidget.AddToViewport` _output_get 0)
  (`WidgetBlueprintLibrary.SetInputMode_UIOnlyEx` (`GameplayStatics.GetPlayerController` 0) (`self.WBP_LobbyHUD`))
  (set `PlayerController.bShowMouseCursor` true (`GameplayStatics.GetPlayerController` 0)))

(fn `SetHostUI`
  (bind _wbp_lobbyhud (`self.WBP_LobbyHUD`)
    (:`then`
      (`/Game/UI/LobbyUI/WBP_LobbyHUD.SetHost` _wbp_lobbyhud))
    (:`else`
      (`KismetSystemLibrary.K2_SetTimer` self "SetHost" 0.1))))

(fn `UpdateIsReady`
  (bind _wbp_lobbyhud (`self.WBP_LobbyHUD`)
    (:`then`
      (`/Game/UI/LobbyUI/WBP_LobbyHUD.UpdateIsReady` _wbp_lobbyhud))
    (:`else`
      (`KismetSystemLibrary.K2_SetTimer` self "UpdateIsReady" 0.1))))

(fn `UpdateUserInfo`
  (bind _wbp_lobbyhud (`self.WBP_LobbyHUD`)
    (:`then`
      (`/Game/UI/LobbyUI/WBP_LobbyHUD.UpdateUserInfo` _wbp_lobbyhud))
    (:`else`
      (`KismetSystemLibrary.K2_SetTimer` self "UpdateUserInfo" 0.2))))

(fn `UpdateUserSelectCharacter`
  (bind _wbp_lobbyhud (`self.WBP_LobbyHUD`)
    (:`then`
      (`/Game/UI/LobbyUI/WBP_LobbyHUD.UpdateUserSelectCharacter` _wbp_lobbyhud))
    (:`else`
      (`KismetSystemLibrary.K2_SetTimer` self "UpdateUserSelectCharacter" 0.2))))

(fn `UserConstructionScript`
  (`parent.UserConstructionScript`))