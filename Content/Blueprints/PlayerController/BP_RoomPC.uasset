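; Player controller for the multiplayer room lobby, handling the player's nickname, GUID, player list and host status.
; The owning client reads the saved nickname from the game instance, and a server event writes it to the room PlayerState and GameMode, keyed by GUID.
; Server events request player list updates through the GameMode, while owner events refresh the room HUD.
; The IsHost RepNotify switches the HUD widget to host UI.
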(event `OwnerUpdatePlayerNickNameFromSave`
  ;[1 1 1] 닉네임
  (bind _nickname (`/Game/Blueprints/BattleEndedGameInstance.GetNickNameFromSaveInfo` (`self.GetBattleEndedGameInstance`)))
  (`self.ServerUpdatePlayerNickName` _nickname))

(event `OwnerdSetPlayerInfo`
  ;[1 1 1] 방 입장
  (`/Game/Blueprints/HUD/BP_RoomHUD.UpdatePlayerInfo` (`self.GetRoomHUD`)))

(event `ServerUpdatePlayerNickName`
  (params (InNickName :type String))
  ;[1 1 1] 닉네임
  (`|ExecutionSequence`
    (:`then_0`
      (set `/Game/Blueprints/PlayerState/BP_RoomPS.NickName` InNickName (`self.GetRoomPS`)))
    (:`then_1`
      (`/Game/Blueprints/GameMode/BP_RoomGM.Set Player Nick Name` (`self.GetRoomGM`) (`self.PlayerGuid`) InNickName))))

(event `ServerUpdatePlayerList`
  (`/Game/Blueprints/GameMode/BP_RoomGM.UpdatePlayerInfo` (`self.GetRoomGM`)))

(event `OwnerUpdatePlayerList`
  (bind _asbp_room_hud (cast `/Game/Blueprints/HUD/BP_RoomHUD` (`self.GetHUD`)))
  (`/Game/Blueprints/HUD/BP_RoomHUD.UpdatePlayerInfo` _asbp_room_hud))

(fn `GetGuid`
  (returns (PlayerGuid :type "Guid Structure"))
  (return (`self.PlayerGuid`)))

(fn `OnRep_IsHost`
  (bind _asbp_room_hud (cast `/Game/Blueprints/HUD/BP_RoomHUD` (`self.GetHUD` (`GameplayStatics.GetPlayerController` 0))))
  (bind _wbp_roomhud (`/Game/Blueprints/HUD/BP_RoomHUD.WBP_RoomHUD` _asbp_room_hud)
    (:`then`
      (`/Game/UI/RoomUI/WBP_RoomHUD.SetHostUI` _wbp_roomhud))
    (:`else`)))

(fn `SetGuid`
  (params (PlayerGuid :type "Guid Structure"))
  (set `self.PlayerGuid` PlayerGuid))

(fn `UserConstructionScript`
  (`parent.UserConstructionScript`))