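; Lobby player controller that links each player to lobby game mode, player state and HUD for nickname, ready, character selection and game start.
; Server-named events update player state or forward to the game mode; owner-named events refresh the HUD.
; Game start saves the game state's player list, and each owner saves its info to the game instance before opening hardcoded 127.0.0.1:7778.
; Host replication retries on a timer until the HUD is valid.
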(event `OwnerSetNickName`
  ;[1 1 1] UserInfo
  (bind _nickname (`/Game/Blueprints/BattleEndedGameInstance.GetNickNameFromSaveInfo` (`self.GetBattleEndedGameInstance`)))
  (`self.ServerSetUserNickName` _nickname))

(event `Server_UpdateReady`
  (params (IsReady :type Boolean) (NewParam :type "Guid Structure"))
  ;[1 1 1] LobbyReadyState
  (`/Game/Blueprints/GameMode/BP_LobbyGM.SetUserReady` (`self.GetLobbyGM`) IsReady NewParam))

(event `Server_GameStart`
  (`|ExecutionSequence`
    (:`then_0`
      (bind _asbp_lobby_gs (cast `/Game/Blueprints/GameState/BP_LobbyGS` (`GameplayStatics.GetGameState`)))
      (`/Game/Blueprints/BattleEndedGameInstance.ServerSaveGS` (`self.GetBattleEndedGameInstance`) (`/Game/Blueprints/GameState/BP_LobbyGS.Player Info Arr` _asbp_lobby_gs)))
    (:`then_1`
      (`/Game/Blueprints/GameMode/BP_LobbyGM.GameStart` (`self.GetLobbyGM`)))))

(event `Owner_UpdateUserReady`
  ;[1 1 1] LobbyReadyState
  (`/Game/Blueprints/HUD/BP_LobbyHUD.UpdateIsReady` (`self.GetLobbyHUD`)))

(event `ServerSetUserNickName`
  (params (InNickName :type String))
  ;[1 1 1] UserInfo
  (set `/Game/Blueprints/PlayerState/BP_LobbyPS.NickName` InNickName (`self.GetLobbyPS`)))

(event `Owner_MoveToInGame`
  (bind _asbp_lobby_ps (`self.GetLobbyPS`))
  (`KismetSystemLibrary.PrintString` "Hello" true true (struct :`G` 0.66 :`B` 1.0 :`A` 1.0) 52.0)
  (`self.MoveToInGame` (`/Game/Blueprints/PlayerState/BP_LobbyPS.NickName` _asbp_lobby_ps) (`/Game/Blueprints/PlayerState/BP_LobbyPS.Guid` _asbp_lobby_ps) (`/Game/Blueprints/PlayerState/BP_LobbyPS.EPlayerClass` _asbp_lobby_ps) (`/Game/Blueprints/PlayerState/BP_LobbyPS.NumOrder` _asbp_lobby_ps) "127.0.0.1:7778"))

(event `ServerUpdateUserList`
  (params (NewParam :type "Guid Structure") (NewParam2 :type String))
  ;[1 1 1] UserInfo
  (`/Game/Blueprints/GameMode/BP_LobbyGM.Set User Info NickName` (`self.GetLobbyGM`) NewParam NewParam2))

(event `OwnerUpdateUserList`
  ;[1 1 1] UserInfo
  (`/Game/Blueprints/HUD/BP_LobbyHUD.UpdateUserInfo` (`self.GetLobbyHUD`)))

(event `Server_SelectWarrior`
  (params (InClass :type "/Game/Character/PlayerCharacter/LobbyPlayerCharacter/BP_LobbyCharacter Class Reference"))
  ;[1 1 1] LobbyCharacter
  (`/Game/Blueprints/GameMode/BP_LobbyGM.UpdateCharacterAnimaion` (`self.GetLobbyGM`) self InClass))

(event `ServerSetUserNum`
  (params (NumOrder :type Integer))
  ;[1 1 1] UserInfo
  (set `/Game/Blueprints/PlayerState/BP_LobbyPS.NumOrder` NumOrder (`self.GetLobbyPS`)))

(event `Server_PlayerCharacterSelect`
  (params (InGuid :type "Guid Structure") (InClass :type "/Game/Enum/EPlayerClass Enum" :default "NewEnumerator2"))
  ;[1 1 1] Character Select
  (`/Game/Blueprints/GameMode/BP_LobbyGM.Set User Select Character` (`self.GetLobbyGM`) InGuid InClass))

(event `ServerUpdateUserNum`
  (params (NewParam :type "Guid Structure") (NumOrder :type Integer))
  ;[1 1 1] Update
  (`KismetSystemLibrary.Delay` 0.1)
  (`/Game/Blueprints/GameMode/BP_LobbyGM.SetUserInfoNum` (`self.GetLobbyGM`) NewParam NumOrder))

(event `Owner_UpdateUserSelectCharacter`
  ;[1 1 1] Character Select
  (`/Game/Blueprints/HUD/BP_LobbyHUD.UpdateUserSelectCharacter` (`self.GetLobbyHUD`)))

(fn `GetLobbyGM`
  (returns (`AsBP Lobby GM` :type "/Game/Blueprints/GameMode/BP_LobbyGM Object Reference"))
  (bind _asbp_lobby_gm (cast `/Game/Blueprints/GameMode/BP_LobbyGM` (`GameplayStatics.GetGameMode`)))
  (return _asbp_lobby_gm))

(fn `GetLobbyHUD`
  (returns (`AsBP Lobby HUD` :type "/Game/Blueprints/HUD/BP_LobbyHUD Object Reference"))
  (bind _asbp_lobby_hud (cast `/Game/Blueprints/HUD/BP_LobbyHUD` (`self.GetHUD`)))
  (return _asbp_lobby_hud))

(fn `GetLobbyPS`
  (returns (`AsBP Lobby PS` :type "/Game/Blueprints/PlayerState/BP_LobbyPS Object Reference"))
  (bind _asbp_lobby_ps (cast `/Game/Blueprints/PlayerState/BP_LobbyPS` (`self.PlayerState`)))
  (return _asbp_lobby_ps))

(fn `MoveToInGame`
  (params (InNickName :type String) (InGuid :type "Guid Structure") (InClass :type "/Game/Enum/EPlayerClass Enum" :default "NewEnumerator2") (InNum :type Integer) (InIP :type String))
  (`/Game/Blueprints/BattleEndedGameInstance.SaveUserInfo` (`self.GetBattleEndedGameInstance`) InNickName InGuid InClass InNum)
  (`GameplayStatics.OpenLevel` (`KismetStringLibrary.Conv_StringToName` (`local.InIP`))))

(fn `OnRep_Is Host`
  (bind _asbp_lobby_hud (`self.GetLobbyHUD`))
  (`/Engine/EditorBlueprintResources/StandardMacros.IsValid` _asbp_lobby_hud
    (:`Is Valid`
      (`/Game/Blueprints/HUD/BP_LobbyHUD.SetHostUI` _asbp_lobby_hud))
    (:`Is Not Valid`
      (`KismetSystemLibrary.K2_SetTimer` self "OnRep_Is Host" 0.1))))

(fn `SetGuid`
  (params (PlayerGuid :type "Guid Structure"))
  (bind _output_get (set `self.Player Guid` PlayerGuid))
  (bind _asbp_lobby_ps (cast `/Game/Blueprints/PlayerState/BP_LobbyPS` (`self.PlayerState`)))
  (set `/Game/Blueprints/PlayerState/BP_LobbyPS.Guid` _output_get _asbp_lobby_ps))

(fn `UserConstructionScript`
  (`parent.UserConstructionScript`))