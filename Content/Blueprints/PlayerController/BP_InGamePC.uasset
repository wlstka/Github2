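; In-game player controller for a networked click-to-move game with light attacks and item pickup.
; The server spawns a BP_Warrior possessed by an AIC_Player at a random PlayerStart, while the client pawn follows it as a camera anchor.
; Held mouse input sends cursor hit locations for AI movement, holding position while IsAttack is set.
; Pickups route by data-table item type to item messages and HUD inventory or equipment refreshes.
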(event `self.ReceiveBeginPlay`
  ;[1 1 1] Begin
  (`KismetSystemLibrary.Delay` 0.2)
  (set `self.bShowMouseCursor` true)
  (`WidgetBlueprintLibrary.SetInputMode_GameAndUIEx` self null "DoNotLock" false))

(event `Server_InitPlayer`
  ;[1 1 1] Init
  (bind _asbp_in_game_pawn (cast `/Game/Character/BP_InGamePawn` (`self.K2_GetPawn`)))
  (bind _output_get (set `self.ClientSide_PawnRef` _asbp_in_game_pawn))
  (bind _output_get_2 (set `/Game/Character/BP_InGamePawn.ClientSide_PCRef` self _output_get))
  (`self.Server_SpawnPlayer` _output_get_2))

(event `InputAction|LightAttack`
  (params (Key :type "Key Structure"))
  ;[1 1 1] Attack
  (:`Pressed`
    (set `self.IsAttack` true)
    (`|ExecutionSequence`
      (:`then_0`
        (`self.Server_LightAttack`))
      (:`then_1`
        (`self.Server_LightAttackDecreaseRP`)))))

(event `InputAction|MouseMove`
  (params (Key :type "Key Structure"))
  (bind _serverside_characterref (`self.ServerSide_CharacterRef`))
  ;[1 1 1] Move
  (:`Pressed`
    (goto _label :!via `Open`))
  (:`Released`
    (goto _label :!via `Close`)))

(event `self.ReceiveTick`
  (params (DeltaSeconds :type "Float (single-precision)"))
  ;[1 1 1] Move
  (`|ExecutionSequence`
    (:`then_0`
      (`self.Client_MouseCapture`))
    (:`then_1`
      (`self.Client_UpdateCamera` DeltaSeconds))))

(event `Client_MouseCapture`
  (bind (_bblockinghit _binitialoverlap _time _distance _location) (`GameplayStatics.BreakHitResult` (`self.GetHitResultUnderCursorByChannel` "TraceTypeQuery1")))
  ;[1 1 1] Move
  (if _bblockinghit
    (set `self.MouseLocation` _location)))

(event `Client_UpdateCamera`
  (params (DeltaTime :type "Float (double-precision)"))
  (bind _serverside_characterref (`self.ServerSide_CharacterRef`))
  ;[1 1 1] Move
  (`/Engine/EditorBlueprintResources/StandardMacros.IsValid` _serverside_characterref
    (:`Is Valid`
      (`self.K2_SetActorLocation` (`self.ClientSide_PawnRef`) (`KismetMathLibrary.VInterpTo` (`self.K2_GetActorLocation` _serverside_characterref) (`self.K2_GetActorLocation` (`self.ClientSide_PawnRef`)) 0.0 10.0) false false))))

(event `Server_MoveServerCharacter`
  (params (InMouse :type "Vector Structure"))
  (bind _serverside_pcref (`self.ServerSide_PCRef`))
  ;[1 1 1] Move
  (`/Engine/EditorBlueprintResources/ActorMacros.Switch Has Authority`
    (:`Authority`
      (if (>= (`KismetMathLibrary.VSize` (- (`self.K2_GetActorLocation` (`self.ServerSide_CharacterRef`)) InMouse)) (`self.MinClickDistance`))
        (`/Engine/EditorBlueprintResources/StandardMacros.IsValid` _serverside_pcref
          (:`Is Valid`
            (`AIController.MoveToLocation` _serverside_pcref InMouse -1.0 true true false true null true)))))))

(event `InputAxis|MouseMove`
  (params (AxisValue :type "Float (single-precision)"))
  (bind _serverside_characterref (`self.ServerSide_CharacterRef`))
  ;[1 1 1] Move
  (`/Engine/EditorBlueprintResources/StandardMacros.Gate` true :!label _label
    (:`Exit`
      (if (not (`self.IsAttack`))
        (`/Engine/EditorBlueprintResources/StandardMacros.IsValid` (`self.ServerSide_CharacterRef`)
          (:`Is Valid`
            (`self.Server_MoveServerCharacter` (`self.MouseLocation`))))
        (else
          (`/Engine/EditorBlueprintResources/StandardMacros.IsValid` _serverside_characterref
            (:`Is Valid`
              (`self.Server_MoveServerCharacter` (`self.K2_GetActorLocation` _serverside_characterref)))))))))

(event `Server_LightAttack`
  ;[1 1 1] Attack
  (bind _asbp_warrior (cast `/Game/Character/PlayerCharacter/BP_Warrior` (`self.ServerSide_CharacterRef`)))
  (`/Game/Character/PlayerCharacter/BP_Warrior.LightAttackCombo` _asbp_warrior))

(event `Server_LightAttackDecreaseRP`
  ;[1 1 1] Attack
  (bind _asbp_warrior (cast `/Game/Character/PlayerCharacter/BP_Warrior` (`self.ServerSide_CharacterRef`)))
  (`/Game/Character/PlayerCharacter/BP_Warrior.LightAttackDecreaseRP` _asbp_warrior))

(event `InputAction|PickUpItem`
  (params (Key :type "Key Structure"))
  (bind _as_bp_item (`self.As BP Item`))
  (bind _returnvalue (`self.GetComponentByClass` _as_bp_item "/Game/Items/BPC_Item.BPC_Item_C"))
  (bind (_datatable _rowname) (break `DataTableRowHandle` (`/Game/Items/BPC_Item.ItemData` _returnvalue)))
  (:`Pressed`
    (`self.PickUpItem`)
    (`/Engine/EditorBlueprintResources/StandardMacros.IsValid` _as_bp_item
      (:`Is Valid`
        (bind _returnvalue_2 (`|GetDataTableRow` _datatable _rowname)
          (:`then`
            (switch `/Game/Enum/EItemType` (`.ItemType_18_C1CA6A1346C452D62E931B8681C9F267` (break `/Game/Items/S_Item` _returnvalue_2))
              (:`NewEnumerator1`
                (message `/Game/Inventory/BPI_Interact.Interact` _returnvalue (`self.ServerSide_CharacterRef`))
                (`self.UpdateInventory`))
              (:`NewEnumerator2`
                (message `/Game/Inventory/BPI_Interact.Test` _returnvalue (`self.ServerSide_CharacterRef`) :!label _label_2)
                (`self.UpdateEquipmentInventory`))
              (:`NewEnumerator3`
                (goto _label_2))
              (:`NewEnumerator5`
                (goto _label_2))
              (:`NewEnumerator4`
                (goto _label_2)))))))))

(event `Server_PickUpItem`
  (params (`타깃` :type "Actor Object Reference"))
  (`self.K2_DestroyActor` `타깃`))

(event `Owner_SetDropItemUI`
  (params (InItem :type "/Game/Items/BP_Item Object Reference") (IsVisibility :type Boolean))
  (`SceneComponent.SetVisibility` (`/Game/Items/BP_Item.Widget` InItem) IsVisibility false))

(event `UpdateInventory`
  (bind _asbp_in_game_hud (cast `/Game/Blueprints/HUD/BP_InGameHUD` (`self.GetHUD`)))
  (bind _wbp_ingamehud (`/Game/Blueprints/HUD/BP_InGameHUD.WBP_InGameHUD` _asbp_in_game_hud))
  (`/Engine/EditorBlueprintResources/StandardMacros.IsValid` _wbp_ingamehud
    (:`Is Valid`
      (`/Game/UI/InGameUI/Inventory/WBP_Inventory.UpdateInventory` (`/Game/UI/InGameUI/WBP_InGameHUD.WBP_Inventory` _wbp_ingamehud) (`/Game/Character/PlayerCharacter/BP_BasePlayerCharacter.BPC_InventorySystem` (`self.ServerSide_CharacterRef`))))))

(event `UpdateEquipmentInventory`
  (bind _asbp_in_game_hud (cast `/Game/Blueprints/HUD/BP_InGameHUD` (`self.GetHUD`)))
  (bind _wbp_ingamehud (`/Game/Blueprints/HUD/BP_InGameHUD.WBP_InGameHUD` _asbp_in_game_hud))
  (`/Engine/EditorBlueprintResources/StandardMacros.IsValid` _wbp_ingamehud
    (:`Is Valid`
      (`/Game/UI/InGameUI/Equipment/WBP_EquipmentInventory.UpdateEquipmentInventory` (`/Game/UI/InGameUI/WBP_InGameHUD.WBP_EquipmentInventory` _wbp_ingamehud) (`/Game/Character/PlayerCharacter/BP_BasePlayerCharacter.BPC_EquipmentSystem` (`self.ServerSide_CharacterRef`))))))

(fn `MoveToHitLocation`
  (params (Hit :type "HitResult Structure (by ref)"))
  (bind (_bblockinghit _binitialoverlap _time _distance _location) (`GameplayStatics.BreakHitResult` Hit))
  (if (>= (`KismetMathLibrary.VSize` (- (`self.K2_GetActorLocation` (`self.K2_GetPawn`)) _location)) (`self.Min Click Distance`))
    (`AIBlueprintHelperLibrary.SimpleMoveToLocation` self _location)))

(fn `PickUpItem`
  (bind _output (`|GetArrayItem` (`self.GetOverlappingActors` (`self.ServerSide_CharacterRef`) "/Game/Items/BP_Item.BP_Item_C")))
  (`/Engine/EditorBlueprintResources/StandardMacros.IsValid` _output
    (:`Is Valid`
      (bind _asbp_item (cast `/Game/Items/BP_Item` _output))
      (set `self.As BP Item` _asbp_item)
      (`self.Server_PickUpItem` _output))))

(fn `Server_SpawnPlayer`
  (bind _clientside_pawnref (`self.ClientSide_PawnRef`))
  (bind _returnvalue (`self.GetTransform` _clientside_pawnref))
  (`/Engine/EditorBlueprintResources/ActorMacros.Switch Has Authority`
    (:`Authority`
      (bind _outactors (`GameplayStatics.GetAllActorsOfClass` "/Script/Engine.PlayerStart"))
      (`/Engine/EditorBlueprintResources/StandardMacros.DoOnce` false
        (:`Completed`
          (`self.K2_SetActorLocation` _clientside_pawnref (`self.K2_GetActorLocation` (`|GetArrayItem` _outactors (`KismetMathLibrary.RandomIntegerInRange` 0 (`KismetArrayLibrary.Array_LastIndex` _outactors)))) false false)
          (bind _returnvalue_2 (`|SpawnActorFromClass` "/Game/Character/PlayerCharacter/BP_Warrior.BP_Warrior_C" _returnvalue "Undefined" "OverrideRootScale" null null))
          (set `self.ServerSide_CharacterRef` _returnvalue_2)
          (bind _asbp_in_game_ps (cast `/Game/Blueprints/PlayerState/BP_InGamePS` (`self.PlayerState`)))
          (set `/Game/Blueprints/PlayerState/BP_InGamePS.ServerSideCharacaterRef` (`self.ServerSide_CharacterRef`) _asbp_in_game_ps)
          (bind _returnvalue_3 (`|SpawnActorFromClass` "/Game/AI/AIC_Player.AIC_Player_C" _returnvalue "Undefined" "OverrideRootScale" self null))
          (bind _output_get (set `self.ServerSide_PCRef` _returnvalue_3))
          (set `/Game/AI/AIC_Player.ServerSide_BasePlayerCharacterRef` (`self.ServerSide_CharacterRef`) _output_get)
          (`self.Possess` (`self.ServerSide_PCRef`) (`self.ServerSide_CharacterRef`)))))))

(fn `UserConstructionScript`
  (`parent.UserConstructionScript`))