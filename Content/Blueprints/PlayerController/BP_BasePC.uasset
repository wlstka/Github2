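; Base player controller that provides typed accessors to framework objects for the room and in-game phases.
; Getters cast the game instance to BattleEndedGameInstance, game mode and HUD to their Room or InGame classes, and game state and player state to Room classes only.
; It holds no other logic: the construction script is empty, and each getter returns its result only when the cast succeeds.
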(fn `GetBattleEndedGameInstance`
  (returns (`AsBattle Ended Game Instance` :type "/Game/Blueprints/BattleEndedGameInstance Object Reference"))
  (bind _asbattle_ended_game_instance (cast `/Game/Blueprints/BattleEndedGameInstance` (`GameplayStatics.GetGameInstance`)))
  (return _asbattle_ended_game_instance))

(fn `GetInGameGM`
  (returns (`AsBP in Game GM` :type "/Game/Blueprints/GameMode/BP_InGameGM Object Reference"))
  (bind _asbp_in_game_gm (cast `/Game/Blueprints/GameMode/BP_InGameGM` (`GameplayStatics.GetGameMode`)))
  (return _asbp_in_game_gm))

(fn `GetInGameHUD`
  (returns (`AsBP in Game HUD` :type "/Game/Blueprints/HUD/BP_InGameHUD Object Reference"))
  (bind _asbp_in_game_hud (cast `/Game/Blueprints/HUD/BP_InGameHUD` (`self.GetHUD`)))
  (return _asbp_in_game_hud))

(fn `GetRoomGM`
  (returns (`AsBP Room GM` :type "/Game/Blueprints/GameMode/BP_RoomGM Object Reference"))
  (bind _asbp_room_gm (cast `/Game/Blueprints/GameMode/BP_RoomGM` (`GameplayStatics.GetGameMode`)))
  (return _asbp_room_gm))

(fn `GetRoomGS`
  (returns (`AsBP Room GS` :type "/Game/Blueprints/GameState/BP_RoomGS Object Reference"))
  (bind _asbp_room_gs (cast `/Game/Blueprints/GameState/BP_RoomGS` (`GameplayStatics.GetGameState`)))
  (return _asbp_room_gs))

(fn `GetRoomHUD`
  (returns (`AsBP Room HUD` :type "/Game/Blueprints/HUD/BP_RoomHUD Object Reference"))
  (bind _asbp_room_hud (cast `/Game/Blueprints/HUD/BP_RoomHUD` (`self.GetHUD`)))
  (return _asbp_room_hud))

(fn `GetRoomPS`
  (returns (`AsBP Room PS` :type "/Game/Blueprints/PlayerState/BP_RoomPS Object Reference"))
  (bind _asbp_room_ps (cast `/Game/Blueprints/PlayerState/BP_RoomPS` (`self.PlayerState`)))
  (return _asbp_room_ps))

(fn `UserConstructionScript`)