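; Equipment system component that holds an owner's equipment slots and places items into them by item type.
; BeginPlay sizes the slot array, gives the first four slots fixed types, then prints each slot for debugging.
; AddEquipment finds the slot whose type matches the item's DT_Item row.
; The helper TEst then overwrites that slot with the item key and hardcoded type and grade, apparently placeholder logic.
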(event `self.ReceiveBeginPlay`
  (`KismetArrayLibrary.Array_Resize` (`self.EquipmentSlotArr`) (`self.EquipmentSize`))
  (`|ExecutionSequence`
    (:`then_0`
      (for (_array_element _array_index) (`self.EquipmentSlotArr`)
        (switch `int` _array_index
          (:`0`
            (bind _structout (setmembers `/Game/Structs/S_EquipmentSlot` :`StructRef` _array_element :`Type` "NewEnumerator2"))
            (`KismetArrayLibrary.Array_Set` (`self.EquipmentSlotArr`) _array_index _structout))
          (:`1`
            (bind _structout_2 (setmembers `/Game/Structs/S_EquipmentSlot` :`StructRef` _array_element :`Type` "NewEnumerator3"))
            (`KismetArrayLibrary.Array_Set` (`self.EquipmentSlotArr`) _array_index _structout_2))
          (:`2`
            (bind _structout_3 (setmembers `/Game/Structs/S_EquipmentSlot` :`StructRef` _array_element :`Type` "NewEnumerator5"))
            (`KismetArrayLibrary.Array_Set` (`self.EquipmentSlotArr`) _array_index _structout_3))
          (:`3`
            (bind _structout_4 (setmembers `/Game/Structs/S_EquipmentSlot` :`StructRef` _array_element :`Type` "NewEnumerator4"))
            (`KismetArrayLibrary.Array_Set` (`self.EquipmentSlotArr`) _array_index _structout_4)))))
    (:`then_1`
      (for _array_element_2 (`self.EquipmentSlotArr`)
        (bind (_name _type _grade) (break `/Game/Structs/S_EquipmentSlot` _array_element_2))
        (`KismetSystemLibrary.PrintString` (`KismetStringLibrary.Concat_StrStr` (`KismetStringLibrary.Conv_NameToString` _name) (`|GetEnumeratorNameAsString` _type) (`|GetEnumeratorNameAsString` _grade)))))))

(event `self.ReceiveTick`
  (params (DeltaSeconds :type "Float (single-precision)")))

(fn `AddEquipment`
  (params (ItemKey :type Name))
  (bind (_array_index _findslot) (`self.FindEquipmentSlot` (`local.ItemKey`)))
  (if _findslot
    (`self.TEst` _array_index (`local.ItemKey`))))

(fn `FindEquipmentSlot`
  (params (ItemKey :type Name))
  (returns (`Array Index` :type Integer) (FindSlot :type Boolean))
  (for (_array_element _array_index) (`self.EquipmentSlotArr`)
    (bind _returnvalue (`|GetDataTableRow` "/Game/Items/DT_Item.DT_Item" ItemKey)
      (:`then`
        (if (`|EnumEquality` (`.ItemType_18_C1CA6A1346C452D62E931B8681C9F267` (break `/Game/Items/S_Item` _returnvalue)) (`.Type_8_324E07594CE8BF5FFC099B90B290DC29` (break `/Game/Structs/S_EquipmentSlot` _array_element)))
          (return _array_index true)
          (else
            (`KismetSystemLibrary.PrintString` "Fail")))))))

(fn `TEst`
  (params (Index :type Integer) (ItemKey :type Name))
  (`KismetArrayLibrary.Array_Set` (`self.EquipmentSlotArr`) Index (make `/Game/Structs/S_EquipmentSlot` ItemKey "NewEnumerator2" "NewEnumerator1")))