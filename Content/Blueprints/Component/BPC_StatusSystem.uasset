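; Status component that tracks a character's HP and RP resources along with a death flag.
; BeginPlay fills both to their maximums, and Tick regenerates RP by a fixed per-frame step, not scaled by delta time, whenever IsAction is false.
; Decrease functions clamp each value at zero, and HP dropping below zero sets IsDead.
; The HP decrease also prints the resulting value.
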(event `self.ReceiveBeginPlay`
  (`self.InitStatus`))

(event `self.ReceiveTick`
  (params (DeltaSeconds :type "Float (single-precision)"))
  (if (not (`self.IsAction`))
    (`self.NaturalRecoveryRP`)))

(fn `DecraseHP`
  (params (In :type "Float (double-precision)"))
  (bind _returnvalue (- (`self.CurHP`) In))
  (`KismetSystemLibrary.PrintString` (`KismetStringLibrary.Conv_DoubleToString` _returnvalue))
  (bind _output_get (set `self.CurHP` _returnvalue))
  (if (< _output_get 0.0)
    (set `self.CurHP` 0.0)
    (set `self.IsDead` true)))

(fn `DecreaseRP`
  (params (In :type "Float (double-precision)"))
  (bind _output_get (set `self.CurRP` (- (`self.CurRP`) In)))
  (if (< _output_get 0.0)
    (set `self.CurRP` 0.0)))

(fn `InitStatus`
  (set `self.CurHP` (`self.MaxHP`))
  (set `self.CurRP` (`self.MaxRP`)))

(fn `NaturalRecoveryRP`
  (bind _output_get (set `self.CurRP` (+ (`self.CurRP`) 0.1)))
  (if (> _output_get (`self.MaxRP`))
    (set `self.CurRP` (`self.MaxRP`))))