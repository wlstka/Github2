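; Anim notify state that runs melee weapon hit detection for BP_Warrior during an animation window.
; Each tick sphere-traces for a single object type between the owner's WeaponBottom and WeaponTop components, with debug drawing left on.
; A hit BP_Warrior receives Damage only if the attacker's IsAttackHit is false, then the flag is set.
; Begin and end both clear the flag, limiting each window to one damaging hit.
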(fn `Received_NotifyBegin`
  (params (MeshComp :type "SkeletalMeshComponent Object Reference") (Animation :type "AnimSequenceBase Object Reference") (TotalDuration :type "Float (double-precision)"))
  (returns (ReturnValue :type Boolean))
  (bind _asbp_warrior (cast `/Game/Character/PlayerCharacter/BP_Warrior` (`ActorComponent.GetOwner` MeshComp)))
  (set `/Game/Character/PlayerCharacter/BP_Warrior.IsAttackHit` false _asbp_warrior)
  (return false))

(fn `Received_NotifyEnd`
  (params (MeshComp :type "SkeletalMeshComponent Object Reference") (Animation :type "AnimSequenceBase Object Reference"))
  (returns (ReturnValue :type Boolean))
  (bind _asbp_warrior (cast `/Game/Character/PlayerCharacter/BP_Warrior` (`ActorComponent.GetOwner` MeshComp)))
  (set `/Game/Character/PlayerCharacter/BP_Warrior.IsAttackHit` false _asbp_warrior)
  (return false))

(fn `Received_NotifyTick`
  (params (MeshComp :type "SkeletalMeshComponent Object Reference") (Animation :type "AnimSequenceBase Object Reference") (FrameDeltaTime :type "Float (double-precision)"))
  (returns (ReturnValue :type Boolean))
  (bind _asbp_warrior (cast `/Game/Character/PlayerCharacter/BP_Warrior` (`ActorComponent.GetOwner` MeshComp)))
  (bind (_outhit _returnvalue) (`KismetSystemLibrary.SphereTraceSingleForObjects` :`WorldContextObject` _asbp_warrior :`Start` (`SceneComponent.K2_GetComponentLocation` (`/Game/Character/PlayerCharacter/BP_Warrior.WeaponBottom` _asbp_warrior)) :`End` (`SceneComponent.K2_GetComponentLocation` (`/Game/Character/PlayerCharacter/BP_Warrior.WeaponTop` _asbp_warrior)) :`Radius` 20.0 :`ObjectTypes` (`|MakeArray` "ObjectTypeQuery7" :!type "EObjectTypeQuery Enum") :`DrawDebugType` "ForDuration" :`DrawTime` 1.0))
  (if _returnvalue
    (bind _asbp_warrior_2 (cast `/Game/Character/PlayerCharacter/BP_Warrior` (`.HitActor` (`GameplayStatics.BreakHitResult` _outhit))))
    (if (not (`/Game/Character/PlayerCharacter/BP_Warrior.IsAttackHit` _asbp_warrior))
      (`/Game/Character/PlayerCharacter/BP_BasePlayerCharacter.Damage` _asbp_warrior_2 (`self.In`))
      (set `/Game/Character/PlayerCharacter/BP_Warrior.IsAttackHit` true _asbp_warrior)
      (return false))))