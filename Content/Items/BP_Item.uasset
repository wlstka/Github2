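; BP_Item is a world item that detects nearby actors with a sphere overlap and toggles drop-item UI.
; Overlap begin and end cast the overlapping actor's owner to AIC_Player and pass it the item with a visibility flag.
; On clients, the item also sets or clears itself on the BP_InGamePC cached at BeginPlay, without checking which actor overlapped.
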(event `self.ReceiveBeginPlay`
  (`/Engine/EditorBlueprintResources/ActorMacros.Switch Has Authority`
    (:`Remote`
      (bind _asbp_in_game_pc (cast `/Game/Blueprints/PlayerController/BP_InGamePC` (`GameplayStatics.GetPlayerController` 0)))
      (set `self.As BP In Game PC` _asbp_in_game_pc))))

(event `self.Sphere.OnComponentBeginOverlap`
  (params (OverlappedComponent :type "PrimitiveComponent Object Reference") (OtherActor :type "Actor Object Reference") (OtherComp :type "PrimitiveComponent Object Reference") (OtherBodyIndex :type Integer) (bFromSweep :type Boolean) (SweepResult :type "HitResult Structure (by ref)"))
  (`self.SetDropItemUI` OtherActor true)
  (`/Engine/EditorBlueprintResources/ActorMacros.Switch Has Authority`
    (:`Remote`
      (set `/Game/Blueprints/PlayerController/BP_InGamePC.As BP Item` self (`self.As BP In Game PC`)))))

(event `self.Sphere.OnComponentEndOverlap`
  (params (OverlappedComponent :type "PrimitiveComponent Object Reference") (OtherActor :type "Actor Object Reference") (OtherComp :type "PrimitiveComponent Object Reference") (OtherBodyIndex :type Integer))
  (`self.SetDropItemUI` OtherActor)
  (`/Engine/EditorBlueprintResources/ActorMacros.Switch Has Authority`
    (:`Remote`
      (set `/Game/Blueprints/PlayerController/BP_InGamePC.As BP Item` null (`self.As BP In Game PC`)))))

(fn `SetDropItemUI`
  (params (InItem :type "Actor Object Reference") (IsVisibility :type Boolean))
  (bind _asaic_player (cast `/Game/AI/AIC_Player` (`self.GetOwner` InItem)))
  (`/Game/AI/AIC_Player.AIC_SetDropItemUI` _asaic_player self IsVisibility))

(fn `UserConstructionScript`)